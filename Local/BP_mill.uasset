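; BP_mill is an animated Wheel of Pain mill prop that spins its parts once play begins.
; A timeline started on BeginPlay drives one track value into the relative rotations each update.
; The small rotator yaws by that value, while the grinder and tier-two rotator take a negated pitch rotation tilted on a fixed roll.
; A RotationSpeed variable and Pi-based math remain unconnected.
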(event EventBeginPlay
  (bind _newtrack_0 (Timeline|Timeline_0 Play)
    (:Update
      (Transformation|SetRelativeRotation (Variables|Default|GetSM_wheel_of_pain_small_rotator) (Math|Rotator|MakeRotator 0.0 0.0 _newtrack_0) false false)
      (Transformation|SetRelativeRotation (Variables|Default|GetSM_wheel_of_pain_small_grinder) (* (Math|Rotator|MakeRotator 9e+01 _newtrack_0 0.0) -1.0) false false))))

(event Collision|EventActorBeginOverlap
  (params (OtherActor :type Actor%20Object%20Reference)))

(event EventTick
  (params (DeltaSeconds :type Float%20%28single-precision%29)))

(fn ConstructionScript)