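; Grape stomping crafting station placeable with an animated thrall worker and sound feedback.
; Adding an item to the thrall inventory or crafting queue loops the stomping animation and plays the Sound and Drip components.
; Removal from either stops both sounds, but only crafting queue removal returns the worker to its initial idle animation.
; GetArtisanThrallInventory exposes the station's thrall inventory.
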(event SignalItemAdded(ThrallInventory)
  (params (index :type Integer) (item :type Game%20Item%20Object%20Reference) (srcInventory :type Item%20Inventory%20Object%20Reference) (srcIndex :type Integer))
  (Components|Animation|PlayAnimation (Variables|Default|GetThrallWorker) "/Game/Mods/brewery_mod/Ani_Grape_Stomping.Ani_Grape_Stomping" true)
  (Class|ConanAudioComponent|Play (Variables|Default|GetSound) 0.0))

(event SignalItemRemoved(ThrallInventory)
  (params (index :type Integer) (item :type Game%20Item%20Object%20Reference) (dstInventory :type Item%20Inventory%20Object%20Reference) (dstIndex :type Integer))
  (Class|ConanAudioComponent|Stop (Variables|Default|GetSound)))

(event SignalItemRemoved(CraftingQueue)
  (params (index :type Integer) (item :type Game%20Item%20Object%20Reference) (dstInventory :type Item%20Inventory%20Object%20Reference) (dstIndex :type Integer))
  (Components|Animation|PlayAnimation (Variables|Default|GetThrallWorker) "/Game/Characters/humans/animations/movement/female/normal/A_normal_idle_3rd_F.A_normal_idle_3rd_F" true)
  (Class|ConanAudioComponent|Stop (Variables|Default|GetSound)))

(event SignalItemAdded(CraftingQueue)
  (params (index :type Integer) (item :type Game%20Item%20Object%20Reference) (srcInventory :type Item%20Inventory%20Object%20Reference) (srcIndex :type Integer))
  (Components|Animation|PlayAnimation (Variables|Default|GetThrallWorker) "/Game/Mods/brewery_mod/Ani_Grape_Stomping.Ani_Grape_Stomping" true)
  (Class|ConanAudioComponent|Play (Variables|Default|GetSound) 0.0))

(event EventBeginPlay
  (|CallParentFunction)
  (Components|Animation|PlayAnimation (Variables|Default|GetThrallWorker) "/Game/Characters/humans/animations/movement/female/normal/A_normal_idle_3rd_F.A_normal_idle_3rd_F" true))

(event Collision|EventActorBeginOverlap
  (params (OtherActor :type Actor%20Object%20Reference)))

(event EventTick
  (params (DeltaSeconds :type Float%20%28single-precision%29)))

(fn ConstructionScript
  (|CallParentFunction))

(fn GetArtisanThrallInventory
  (return (Variables|Default|GetThrallInventory)))