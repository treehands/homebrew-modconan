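; Crafting station Blueprint for a fern crop that visually grows over time.
; Outside dedicated servers, a looping one-second timer advances a local counter and linearly scales nine static meshes from a minimum size, restarting after a hard-coded 500 seconds.
; The growth is cosmetic with no replication or saved state in these graphs, and each tick prints debug values.
; It also exposes its thrall inventory through GetArtisanThrallInventory.
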(event Custom|CustomEvent_0
  (bind _output_get (Variables|Default|Settime (+ (Variables|Default|Gettime) 1.0)))
  ;[1 1 1] if > 500 secs reset time
  (if (> _output_get 5e+02)
    (Variables|Default|Settime 0.0)
    (Variables|Default|Setscale (Variables|Default|Getminscale))
    (else
      (Variables|Default|Setscale (+ (* (/ (Variables|Default|Getmaxgrow) (Variables|Default|Getmaxtime)) (Variables|Default|Gettime)) (Variables|Default|Getminscale)))))
  (Transformation|SetRelativeScale3D (Variables|Default|GetStaticMesh5) (Math|Vector|MakeVector (Variables|Default|Getscale) (Variables|Default|Getscale) (Variables|Default|Getscale)))
  (Development|PrintString (Utilities|String|ToString(Float) (Variables|Default|Getscale)))
  (Development|PrintString (Utilities|String|ToString(Float) (Variables|Default|Getscale)))
  (Development|PrintString (Utilities|String|ToString(Float) (Variables|Default|Gettime)))
  (Development|PrintString (Utilities|String|ToString(Float) (Variables|Default|Gettime))))

(event EventBeginPlay
  (|CallParentFunction)
  (if (not (Networking|IsDedicatedServer))
    (Utilities|Time|SetTimerbyEvent (delegate Custom|CustomEvent_0) 1.0 true)))

(fn ConstructionScript
  (|CallParentFunction))

(fn GetArtisanThrallInventory
  (return (Variables|Default|GetThrallInventory)))