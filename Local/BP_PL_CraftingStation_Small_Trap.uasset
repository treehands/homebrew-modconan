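; Small trap crafting station placeable that visually acts out catching a rabbit as its crafting and inventory change.
; Adding an inventory item shows the bait, and removing one restores the set-trap meshes.
; An item leaving the crafting queue reveals a rabbit mesh, then after a delay swaps to the sprung trap with caught rabbit and staggered zap and rabbit sounds.
; The artisan thrall inventory getter returns ThrallInventory.
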(event SignalItemAdded(PlaceableInventory)
  (params (index :type Integer) (item :type Game%20Item%20Object%20Reference) (srcInventory :type Item%20Inventory%20Object%20Reference) (srcIndex :type Integer))
  (Rendering|SetVisibility (Variables|Default|GetSM_Rabbit_Bait) true false))

(event SignalItemRemoved(PlaceableInventory)
  (params (index :type Integer) (item :type Game%20Item%20Object%20Reference) (dstInventory :type Item%20Inventory%20Object%20Reference) (dstIndex :type Integer))
  (Rendering|SetVisibility (Variables|Default|GetSK_rabbit) false false)
  (Rendering|SetVisibility (Variables|Default|GetStaticMesh) true false))

(event SignalItemRemoved(CraftingQueue)
  (params (index :type Integer) (item :type Game%20Item%20Object%20Reference) (dstInventory :type Item%20Inventory%20Object%20Reference) (dstIndex :type Integer))
  (Rendering|SetVisibility (Variables|Default|GetSK_rabbit1_0) true false)
  (Utilities|FlowControl|Delay 5.0)
  (Variables|Default|SetCraftingQueue (Variables|Default|GetCraftingQueue))
  (Rendering|SetVisibility (Variables|Default|GetSK_rabbit) true false)
  (Rendering|SetVisibility (Variables|Default|GetStaticMesh) false false)
  (Class|ConanAudioComponent|Play (Variables|Default|Getnpc_rabbit_trap_zap) 0.0)
  (Utilities|FlowControl|Delay 0.2)
  (Class|ConanAudioComponent|Play (Variables|Default|Getnpc_rabbit_sound) 0.0))

(event EventBeginPlay
  (|CallParentFunction)
  (Class|ConanAudioComponent|Stop (Variables|Default|Getnpc_rabbit_sound)))

(event Collision|EventActorBeginOverlap
  (params (OtherActor :type Actor%20Object%20Reference)))

(event EventTick
  (params (DeltaSeconds :type Float%20%28single-precision%29)))

(fn ConstructionScript
  (|CallParentFunction))

(fn GetArtisanThrallInventory
  (return (Variables|Default|GetThrallInventory)))