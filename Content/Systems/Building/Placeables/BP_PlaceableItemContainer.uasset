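; Placeable item container in the building system, with an inventory and an interaction UI.
; On BeginPlay, after the parent logic, it spawns a game item from its source template ID and, if valid, uses that item's container size stat as the PlaceableInventory's maximum item count.
; It overrides the interactable UI module name to select the ContainerInfo module.
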(event EventBeginPlay
  (|CallParentFunction)
  (bind _returnvalue (Class|GameItemSpawner|SpawnGameItem (Variables|Default|GetSourceItemTemplateID)))
  (Utilities|IsValid _returnvalue
    (:Is%20Valid
      (Class|ItemInventory|SetMaxItemCount (Variables|Default|GetPlaceableInventory) (Class|GameItem|GetIntStat _returnvalue "ItemContainerSize")))))

(event EventActorBeginOverlap
  (params (OtherActor :type Actor%20Object%20Reference)))

(event EventTick
  (params (DeltaSeconds :type Float%20%28single-precision%29)))

(fn ConstructionScript
  (|CallParentFunction))

(fn InteractableGetUIModuleName
  (return "ContainerInfo"))